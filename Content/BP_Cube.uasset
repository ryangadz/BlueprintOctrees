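; BP_Cube is an actor that builds instanced cubes at construction time, subdividing where its volume overlaps WorldStatic objects.
; The construction script sets the mesh and material, clamps the iteration count, and box-tests the volume around the actor.
; An overlap passes the instanced mesh to an Octree function, subject to a minimum-size check.
; With no overlap, it adds one cube instance scaled from the maximum size.
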(event EventBeginPlay)

(event Collision|EventActorBeginOverlap
  (params (OtherActor :type Actor%20Object%20Reference)))

(event EventTick
  (params (DeltaSeconds :type Float%20%28single-precision%29)))

(fn ConstructionScript
  (bind _sizemax (Variables|Default|GetSizeMax))
  (bind _cubeinstance (Variables|Default|GetCubeInstance))
  (Components|StaticMesh|SetStaticMesh _cubeinstance (Variables|Default|GetMesh))
  (Rendering|Material|SetMaterial _cubeinstance 0 (Variables|Default|GetMaterial))
  (Variables|Default|SetIterationsMax (Math|Integer|Clamp(Integer) (Variables|Default|GetIterationsMax) 0 5))
  (Variables|Default|SetCurrentSize _sizemax)
  (bind _output_get (Variables|Default|SetCurrentLoc (Transformation|GetActorLocation)))
  (bind _returnvalue (Collision|BoxOverlapComponents _output_get (Math|Conversions|ToVector(Float) (/ _sizemax 2.0)) (Utilities|Array|MakeArray "ObjectTypeQuery1") 0 0 :!class /Script/Engine.KismetSystemLibrary))
  (if _returnvalue
    (if (< (/ (Variables|Default|GetSizeMax) (Math|Float|Power 2.0 (* (Variables|Default|GetIterationsMax) 2.0))) (/ (Variables|Default|GetCurrentSize) 2.0))
      (CallFunction|Octree (Variables|Default|GetSizeMax) (Variables|Default|GetIterationsMax) (Variables|Default|GetCurrentSize) (Variables|Default|GetCurrentLoc) (Variables|Default|GetCubeInstance)))
    (else
      (Class|InstancedStaticMeshComponent|AddInstanceWorldSpace (Variables|Default|GetCubeInstance) (Math|Transform|MakeTransform (Variables|Default|GetCurrentLoc) "0, 0, 0" (Math|Conversions|ToVector(Float) (/ (Variables|Default|GetSizeMax) 8.0)))))))