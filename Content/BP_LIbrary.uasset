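; BP_LIbrary holds a recursive Octree function that fills space free of WorldStatic geometry with cube instances.
; Each call halves the size and box-tests eight child cells.
; Clear cells become scaled instances on the supplied instanced mesh, so open space gets the largest cubes possible.
; Blocked cells recurse until a size limit derived from MaxSize and MaxIterations, then stay empty.
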(fn Octree
  (params (MaxSize :type Float%20%28single-precision%29) (MaxIterations :type Integer) (Size :type Float%20%28single-precision%29) (Location :type Vector) (InstancedMesh :type Instanced%20Static%20Mesh%20Component%20Object%20Reference))
  ;[1 1 1] Subdivide previous size by 2
  (LocalVariables|SetCurrentSizeL (/ Size 2.0))
  ;[1 1 1] Loop through all locations of subdivided cubes
  (for _index (range 0 7)
    (bind _output_get (LocalVariables|SetCurrentLocL (+ (* (Utilities|Array|Get(acopy) (LocalVariables|GetSubdivided) _index) (LocalVariables|GetCurrentSizeL)) Location)))
    (bind _returnvalue (Collision|BoxOverlapComponents 0 _output_get (Math|Conversions|ToVector(Float) (/ (LocalVariables|GetCurrentSizeL) 2.0)) (Utilities|Array|MakeArray "ObjectTypeQuery1") 0 :!class /Script/Engine.KismetSystemLibrary))
    (if _returnvalue
      ;[1 1 1] Further subdivide and repeat if necessary
      (if (< (/ MaxSize (Math|Float|Power 2.0 (Math|Conversions|ToFloat(Integer) (+ MaxIterations 1)))) (/ (LocalVariables|GetCurrentSizeL) 2.0))
        (CallFunction|Octree MaxSize MaxIterations (LocalVariables|GetCurrentSizeL) (LocalVariables|GetCurrentLocL) InstancedMesh))
      (else
        ;[1 1 1] Add cube if space is clear
        (Class|InstancedStaticMeshComponent|AddInstanceWorldSpace InstancedMesh (Math|Transform|MakeTransform (LocalVariables|GetCurrentLocL) "0, 0, 0" (Math|Conversions|ToVector(Float) (/ (LocalVariables|GetCurrentSizeL) 8.0))))))))